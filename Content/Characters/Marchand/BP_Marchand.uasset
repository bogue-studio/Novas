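; BP_Marchand is a merchant that opens a shop when the player character enters its Box trigger.
; On overlap it prints a greeting and blends the player's view target to itself.
; After a delay slightly longer than the blend, it creates the WB_Shop widget, switches input to UI only, ignores move input and shows the mouse cursor.
; Nothing in this Blueprint restores the view or input afterwards.
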(event `self.Box.OnComponentBeginOverlap`
  (params (OverlappedComponent :type "PrimitiveComponent Object Reference") (OtherActor :type "Actor Object Reference") (OtherComp :type "PrimitiveComponent Object Reference") (OtherBodyIndex :type Integer) (bFromSweep :type Boolean) (SweepResult :type "HitResult Structure (by ref)"))
  (bind _returnvalue (`GameplayStatics.GetPlayerController` 0))
  (if (== OtherActor (`GameplayStatics.GetPlayerCharacter` 0))
    (`KismetSystemLibrary.PrintString` "Hello")
    (`PlayerController.SetViewTargetWithBlend` (`GameplayStatics.GetPlayerController` 0) self 2.0 "VTBlend_Linear" 0.0 false)
    (`KismetSystemLibrary.Delay` 2.2)
    (bind _returnvalue_2 (`|CreateWidget` "/Game/Characters/Marchand/Widget/WB_Shop.WB_Shop_C"))
    (`UserWidget.AddToViewport` _returnvalue_2 0)
    (`WidgetBlueprintLibrary.SetInputMode_UIOnlyEx` _returnvalue null)
    (`Controller.SetIgnoreMoveInput` _returnvalue true)
    (set `PlayerController.bShowMouseCursor` true _returnvalue)))

(fn `UserConstructionScript`)